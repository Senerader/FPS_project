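; Infinite terrain game mode that chains tiles into an endless level and tracks score.
; On begin play it fills a nav mesh volume pool, then spawns a starting run of tiles.
; Each spawned tile receives the shared pool and supplies the attach transform where the next tile spawns.
; Entering a new tile adds a fixed amount to the score.
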(event `self.ReceiveBeginPlay`
  (`self.PopulateVolumePool`)
  (for _ (range 4)
    (`self.SpawnTile`)))

(fn `OnNewTileEnter`
  (set `self.Score` (+ 100.0 (`self.Score`))))

(fn `SpawnTile`
  (bind _returnvalue (`|SpawnActorFromClass` "/Game/Dynamic/Terrain/Tile.Tile_C" (`self.TransformValue`) "Undefined" "OverrideRootScale" null null))
  (`Tile.SetNavMeshPool` _returnvalue (`self.NavMeshVolumePool`))
  (bind _attachtransform (`/Game/Dynamic/Terrain/Tile.GetAttachTransform` _returnvalue))
  (set `self.TransformValue` _attachtransform))

(fn `UserConstructionScript`)