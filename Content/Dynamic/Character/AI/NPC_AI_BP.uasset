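; NPC AI controller Blueprint that runs a guard behavior tree and tracks sensed targets.
; On BeginPlay it sets up the PatrolData blackboard, starts GuardBehaviour and caches the blackboard component.
; AI perception updates write any sensed actor lacking the "Enemy" tag to the KeyEnemy entry, and clear it when such an actor is no longer sensed.
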(event `self.ReceiveBeginPlay`
  (bind _blackboardcomponent (`self.UseBlackboard` "/Game/Dynamic/Character/AI/PatrolData.PatrolData"))
  (`self.RunBehaviorTree` "/Game/Dynamic/Character/AI/GuardBehaviour.GuardBehaviour")
  (set `self.BlackboardComp` _blackboardcomponent))

(event `self.AIPerception.OnTargetPerceptionUpdated`
  (params (Actor :type "Actor Object Reference") (Stimulus :type "AIStimulus Structure"))
  (`self.UpdateBlackboardKey` Actor Stimulus Actor))

(fn `UpdateBlackboardKey`
  (params (ObjectValue :type "Object Object Reference") (AIStimulus :type "AIStimulus Structure (by ref)") (self2 :type "Actor Object Reference"))
  (if (`self.ActorHasTag` self2 "Enemy")
    _
    (elif (`.bSuccessfullySensed` (break `AIStimulus` AIStimulus))
      (`BlackboardComponent.SetValueAsObject` (`self.BlackboardComp`) (`self.KeyEnemy`) ObjectValue)
      (else
        (`BlackboardComponent.ClearValue` (`self.BlackboardComp`) (`self.KeyEnemy`))))))

(fn `UserConstructionScript`)