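; AI controller for guard NPCs that runs the GuardBehaviour behavior tree on the PatrolData blackboard.
; AI perception writes any sensed actor without the "Enemy" tag to the enemy key and clears the key when sensing is lost.
; Each tick, it sets the controlled TP_character's aiming and shooting flags according to whether the controller has a valid focus actor.
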(event `self.ReceiveBeginPlay`
  (bind _blackboardcomponent (`self.UseBlackboard` "/Game/Dynamic/NPC/AI/PatrolData.PatrolData"))
  (`self.RunBehaviorTree` "/Game/Dynamic/NPC/AI/GuardBehaviour.GuardBehaviour")
  (set `self.BlackboardComp` _blackboardcomponent))

(event `self.AIPerception.OnTargetPerceptionUpdated`
  (params (Actor :type "Actor Object Reference") (Stimulus :type "AIStimulus Structure"))
  (if (`self.ActorHasTag` Actor "Enemy")
    _
    (elif (`.bSuccessfullySensed` (break `AIStimulus` Stimulus))
      (`BlackboardComponent.SetValueAsObject` (`self.BlackboardComp`) (`self.KeyEnemy`) Actor)
      (else
        (`BlackboardComponent.ClearValue` (`self.BlackboardComp`) (`self.KeyEnemy`))))))

(event `self.ReceiveTick`
  (params (DeltaSeconds :type "Float (single-precision)"))
  (bind _returnvalue (`KismetSystemLibrary.IsValid` (`self.GetFocusActor`)))
  (bind _astp_character (cast `/Game/Dynamic/NPC/Behaviour/TP_character` (`self.K2_GetPawn`)))
  (set `/Game/Dynamic/NPC/Behaviour/TP_character.AimingBP` _returnvalue _astp_character)
  (set `/Game/Dynamic/NPC/Behaviour/TP_character.ShootingBP` _returnvalue _astp_character))

(fn `UserConstructionScript`)