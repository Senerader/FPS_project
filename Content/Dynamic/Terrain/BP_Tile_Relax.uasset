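; BP_Tile_Relax is an infinite terrain tile with a level gate that locks once the player has passed through it.
; The barrier starts with passable green visuals and a tinted dynamic particle material.
; When the player stops overlapping the gate, it turns red and blocking, shifts a mesh, and notifies BP_InfiniteTerrainGamemode, with a flag limiting notification to once.
; GetAttachTransform exposes the Arrow's world transform as an attach point.
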(event `self.ReceiveBeginPlay`
  (bind _barrierparticles (`self.BarrierParticles`))
  (`self.Unlock`)
  (bind _returnvalue (`KismetMaterialLibrary.CreateDynamicMaterialInstance` "/Game/Dynamic/Terrain/Textures/BarrierMaterial.BarrierMaterial"))
  (bind _output_get (set `self.BarrierParticles` _returnvalue))
  (`PrimitiveComponent.SetMaterial` (`self.ParticleSystem`) 0 _output_get)
  (`MaterialInstanceDynamic.SetVectorParameterValue` _barrierparticles "Color" (struct :`R` 0.456733 :`G` 1.0 :`B` 0.705991 :`A` 0.8))
  (`PrimitiveComponent.SetMaterial` (`self.ParticleSystem`) 0 _barrierparticles))

(event `self.LevelGate.OnComponentEndOverlap`
  (params (OverlappedComponent :type "PrimitiveComponent Object Reference") (OtherActor :type "Actor Object Reference") (OtherComp :type "PrimitiveComponent Object Reference") (OtherBodyIndex :type Integer))
  (bind _barrierparticles (`self.BarrierParticles`))
  (if (== OtherActor (`GameplayStatics.GetPlayerCharacter` 0))
    (`self.Lock`)
    (`self.HasEnteredNewTile`)
    (`SceneComponent.K2_AddRelativeLocation` (`self.StaticMesh111`) (-75.0 0.0 0.0) false false)
    (`MaterialInstanceDynamic.SetVectorParameterValue` _barrierparticles "Color" (struct :`R` 0.338542 :`A` 0.8))
    (`PrimitiveComponent.SetMaterial` (`self.ParticleSystem`) 0 _barrierparticles)))

(fn `GetAttachTransform`
  (returns (AttachTransform :type "Transform Structure"))
  (return (`SceneComponent.K2_GetComponentToWorld` (`self.Arrow`))))

(fn `HasEnteredNewTile`
  (if (not (`self.HasEnteredTile`))
    (bind _asbp_infinite_terrain_gamemode (cast `/Game/Dynamic/BP_InfiniteTerrainGamemode` (`GameplayStatics.GetGameMode`)))
    (`/Game/Dynamic/BP_InfiniteTerrainGamemode.OnNewTileEnter` _asbp_infinite_terrain_gamemode)
    (set `self.HasEnteredTile` true)))

(fn `Lock`
  (bind _staticmesh (`self.StaticMesh`))
  (`PrimitiveComponent.SetCollisionProfileName` _staticmesh "BlockAll")
  (`PrimitiveComponent.SetMaterial` _staticmesh 0 "/Game/Dynamic/Terrain/RedBarrier.RedBarrier"))

(fn `Unlock`
  (bind _staticmesh (`self.StaticMesh`))
  ;[1 1 1] Hardcoded value!
  (`PrimitiveComponent.SetCollisionProfileName` _staticmesh "Barrier")
  (`PrimitiveComponent.SetMaterial` _staticmesh 0 "/Game/Dynamic/Terrain/GreenBarrier.GreenBarrier"))

(fn `UserConstructionScript`)